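; Player character Blueprint for the arrow game that shows a crosshair and shifts the camera while aiming a bow.
; BeginPlay creates the crosshair widget and caches the camera boom's initial socket offset.
; Each Tick, if the equipped weapon is a BP_Bow, its IsAiming flag plays or reverses a timeline.
; The timeline's alpha blends the boom offset toward the aim offset using VectorSlerpNormals rather than a linear lerp.
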(event Collision|EventActorBeginOverlap
  (params (OtherActor :type Actor%20Object%20Reference)))

(event EventTick
  (params (DeltaSeconds :type Float%20%28single-precision%29))
  (bind _asbp_bow (Utilities|Casting|CastToBP_Bow (Variables|Default|GetEquippedWeapon)))
  (if (Variables|/Script/ArrowGame.Bow|GetbIsAiming _asbp_bow)
    (bind _aimalpha (Timeline|AimCameraTimeline Play)
      (:Update
        (Variables|/Script/Engine.SpringArmComponent|SetSocketOffset (Variables|Default|GetCameraBoom) (Class|KismetMathLibrary|VectorSlerpNormals (Variables|Default|GetInitialBoomOffset) (Variables|Default|GetAimBoomOffset) _aimalpha))))
    (else
      (Timeline|AimCameraTimeline Reverse))))

(event EventBeginPlay
  (bind _returnvalue (UserInterface|CreateWidget "/Game/ArrowGame/UI/WBP_Crosshair.WBP_Crosshair_C"))
  (UserInterface|Viewport|AddtoViewport _returnvalue 0)
  (Variables|Default|SetInitialBoomOffset (Variables|/Script/Engine.SpringArmComponent|GetSocketOffset (Variables|Default|GetCameraBoom))))

(fn ConstructionScript)